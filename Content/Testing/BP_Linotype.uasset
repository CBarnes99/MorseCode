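; BP_Linotype is a test interactable typewriter-style actor that takes typed text and displays it on an output widget component.
; On BeginPlay it binds to the type-finished event of the WBP_Letters input widget, and interacting switches to UI-only input focused on its text field.
; Finished text is appended to NewText in a freshly created WBP_OutputText, game input is restored and the letters widget resets.
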(event Custom|Stuff
  (params (Finished%20Text :type Text))
  (CallFunction|TextFinished1 Finished%20Text)
  (Default|Reset (Variables|Default|GetAs%20WBP%20Letters)))

(event EventBeginPlay
  (bind _aswbp_letters (Utilities|Casting|CastToWBP_Letters (UserInterface|GetWidget (Variables|Default|GetInputText))))
  (bind _output_get (Variables|Default|SetAs%20WBP%20Letters _aswbp_letters))
  (EventDispatchers|BindEventtoTypeFinished _output_get (EventDispatchers|CreateEvent :!event Custom|Stuff)))

(event EventBPInteract
  (params (interactor :type Actor%20Object%20Reference))
  (Input|SetInputModeUIOnly (Game|GetPlayerController 0) (Variables|/Game/Testing/WBP_Letters.WBP_Letters_C|GetLetterText (Variables|Default|GetAs%20WBP%20Letters)) "DoNotLock" false))

(fn ConstructionScript)

(fn TextFinished1
  (params (Finished%20Text :type Text))
  (Development|PrintString (Utilities|String|ToString(Text) Finished%20Text))
  (bind _returnvalue (UserInterface|CreateWidget "/Game/Testing/WBP_OutputText.WBP_OutputText_C" 0 (Utilities|Text|FormatText "{a}{b}" (LocalVariables|GetNewText) Finished%20Text)))
  (UserInterface|SetWidget (Variables|Default|GetOutputText) _returnvalue)
  (Input|SetInputModeGameOnly (Game|GetPlayerController 0) false)
  (Development|PrintString "Hello"))